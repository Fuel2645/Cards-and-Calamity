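; BP_SaveGameOBJ is a save game object that stores a game instance reference as a named save.
; Its SaveGame event loads BP_MasterSaveGame from the MASTER slot, adds the new save name to its list, and writes the master's SaveGameRef back to that slot.
; It then creates a fresh BP_SaveGameOBJ, sets SavedInstance to the passed game instance, and saves it under the given name.
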(event Custom|Save%20Game
  (params (Game%20Instance :type Game%20Instance%20Object%20Reference) (Game%20Save%20Name :type String))
  (bind _returnvalue (SaveGame|LoadGamefromSlot "MASTER"))
  (bind _asbp_master_save_game (Utilities|Casting|CastToBP_MasterSaveGame _returnvalue))
  (Utilities|Array|Add (Variables|/Game/ShikanokoKoshtantan/Blueprints/BP_MasterSaveGame.BP_MasterSaveGame_C|GetSave%20Games _asbp_master_save_game) Game%20Save%20Name)
  (bind _output_get (Variables|/Game/ShikanokoKoshtantan/Blueprints/BP_MasterSaveGame.BP_MasterSaveGame_C|SetSave%20Games _asbp_master_save_game (Variables|/Game/ShikanokoKoshtantan/Blueprints/BP_MasterSaveGame.BP_MasterSaveGame_C|GetSave%20Games _asbp_master_save_game)))
  (Variables|/Game/ShikanokoKoshtantan/Blueprints/BP_MasterSaveGame.BP_MasterSaveGame_C|SetSave%20Games (Variables|/Game/ShikanokoKoshtantan/Blueprints/BP_MasterSaveGame.BP_MasterSaveGame_C|GetSave%20Game%20Ref _asbp_master_save_game) _output_get)
  (SaveGame|SaveGametoSlot (Variables|/Game/ShikanokoKoshtantan/Blueprints/BP_MasterSaveGame.BP_MasterSaveGame_C|GetSave%20Game%20Ref _asbp_master_save_game) "MASTER")
  (bind _returnvalue_2 (SaveGame|CreateSaveGameObject "BP_SaveGameOBJ_C"))
  (Variables|BP_SaveGameOBJ_C|SetSaved%20Instance _returnvalue_2 Game%20Instance)
  (SaveGame|SaveGametoSlot _returnvalue_2 Game%20Save%20Name))