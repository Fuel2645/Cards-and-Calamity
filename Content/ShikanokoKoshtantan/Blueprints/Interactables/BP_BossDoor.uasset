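; BP_BossDoor is an interactable door that is removed once the required number of keys has been collected.
; On Interact, it reads the Keys collection from the GI_test game instance and compares its length to NumOfKeysRequired.
; An exact match destroys the door actor, while any other count prints a "not enough" debug message.
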(event EventBeginPlay
  (|CallParentFunction) ; This node is disabled and will not be called.\nDrag off pins to build functionality.
)

(event Collision|EventActorBeginOverlap
  (params (OtherActor :type Actor%20Object%20Reference))
  (|CallParentFunction OtherActor) ; This node is disabled and will not be called.\nDrag off pins to build functionality.
)

(event EventTick
  (params (DeltaSeconds :type Float%20%28single-precision%29))
  (|CallParentFunction DeltaSeconds) ; This node is disabled and will not be called.\nDrag off pins to build functionality.
)

(event EventInteract
  (bind _asgi_test (Utilities|Casting|CastToGI_test (Game|GetGameInstance)))
  (if (== (Utilities|Array|Length (Variables|/Game/Patryk_Klich/GameMode/GI_test.GI_test_C|GetKeys _asgi_test)) (Variables|Default|GetNumOfKeysRequired))
    (Actor|DestroyActor)
    (else
      (Development|PrintString "Not Enoguh Stings"))))

(fn ConstructionScript
  (|CallParentFunction))