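; Player character Blueprint handling movement, yaw look, interaction, health and random rune offers.
; BeginPlay adds the Enhanced Input context, creates the WBP_Temp widget and caches every DT_Runes row.
; Interact line-traces forward to message BP_Interactable actors; health gains are clamped, while a temporary input subtracts health.
; RuneGeneration reveals widget elements, rerolls owned runes and tints the image from a random draw, re-evaluated separately from the ownership check.
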(event Input|EnhancedActionEvents|EnhancedInputActionIA_Interact
  (params (ActionValue :type Boolean) (ElapsedSeconds :type Float%20%28double-precision%29) (TriggeredSeconds :type Float%20%28double-precision%29) (InputAction :type Input%20Action%20Object%20Reference :default "/Game/ShikanokoKoshtantan/Blueprints/IA_Interact.IA_Interact"))
  (bind _returnvalue (Transformation|GetActorLocation))
  (bind _outhit (Collision|LineTraceByChannel _returnvalue (+ _returnvalue (* (Transformation|GetActorForwardVector) 1e+06)) "TraceTypeQuery1" false 0 "None"))
  (if (Utilities|ClassIsChildOf (Utilities|GetClass (.hitactor _outhit)) "/Game/ShikanokoKoshtantan/Blueprints/Interactables/BP_Interactable.BP_Interactable_C")
    (Class|BPIInteract|Interact(Message) (.hitactor _outhit))))

(event Input|EnhancedActionEvents|EnhancedInputActionIA_Tesmp
  (params (ActionValue :type Boolean) (ElapsedSeconds :type Float%20%28double-precision%29) (TriggeredSeconds :type Float%20%28double-precision%29) (InputAction :type Input%20Action%20Object%20Reference :default "/Game/ShikanokoKoshtantan/Blueprints/IA_Tesmp.IA_Tesmp"))
  (:Triggered
    (Utilities|FlowControl|DoOnce false :!label _label
      (:Completed
        (Variables|Default|SetHealth (- (Variables|Default|GetHealth) 5))
        (goto _label Reset)))))

(event Input|EnhancedActionEvents|EnhancedInputActionIA_Look
  (params (ActionValue :type Vector%202D%20Structure) (ElapsedSeconds :type Float%20%28double-precision%29) (TriggeredSeconds :type Float%20%28double-precision%29) (InputAction :type Input%20Action%20Object%20Reference :default "/Game/JJ-TheBest/IA_Look.IA_Look"))
  (Pawn|Input|AddControllerYawInput (.x ActionValue)))

(event Input|EnhancedActionEvents|EnhancedInputActionIA_Movement
  (params (ActionValue :type Vector%202D%20Structure) (ElapsedSeconds :type Float%20%28double-precision%29) (TriggeredSeconds :type Float%20%28double-precision%29) (InputAction :type Input%20Action%20Object%20Reference :default "/Game/JJ-TheBest/IA_Movement.IA_Movement"))
  (bind _returnvalue (Pawn|GetControlRotation :!class /Script/Engine.Pawn))
  (Pawn|Input|AddMovementInput (Math|Vector|GetRightVector (Math|Rotator|MakeRotator (.roll _returnvalue) 0.0 (.yaw _returnvalue))) (.x ActionValue) false)
  (Pawn|Input|AddMovementInput (Math|Vector|GetForwardVector (Math|Rotator|MakeRotator 0.0 0.0 (.yaw (Pawn|GetControlRotation :!class /Script/Engine.Pawn)))) (.y ActionValue) false))

(event EventAddHealth
  (params (Health%20to%20Gain :type Integer))
  (Variables|Default|SetHealth (Math|Integer|Clamp(Integer) (+ Health%20to%20Gain (Variables|Default|GetHealth)) 0 (Variables|Default|GetMax%20Health))))

(event EventBeginPlay
  (bind _asplayer_controller (Utilities|Casting|CastToPlayerController (Pawn|GetController)))
  (Utilities|IsValid (PlayerController|LocalPlayerSubsystems|GetEnhancedInputLocalPlayerSubsystem _asplayer_controller)
    (:Is%20Valid
      (Input|AddMappingContext (PlayerController|LocalPlayerSubsystems|GetEnhancedInputLocalPlayerSubsystem _asplayer_controller) "/Game/JJ-TheBest/IMC_Inputs.IMC_Inputs" 0 "(bIgnoreAllPressedKeysUntilRelease=True,bForceImmediately=False,bNotifyUserSettings=False)")
      (bind _returnvalue (UserInterface|CreateWidget "/Game/ShikanokoKoshtantan/Blueprints/Interactables/WBP_Temp.WBP_Temp_C"))
      (bind _output_get (Variables|Default|SetNewVar _returnvalue))
      (UserInterface|Viewport|AddtoViewport _output_get 0)
      (bind _outcolumnnames (Class|DataTableFunctionLibrary|GetDataTableColumnNames "/Game/ShikanokoKoshtantan/DataValues/Runes/DT_Runes.DT_Runes"))
      (for _array_element _outcolumnnames
        (bind _returnvalue_2 (Utilities|GetDataTableRow "/Game/ShikanokoKoshtantan/DataValues/Runes/DT_Runes.DT_Runes" _array_element)
          (:then
            (Utilities|Array|Add (Variables|Default|GetRunes) _returnvalue_2)))))))

(event EventTick
  (params (DeltaSeconds :type Float%20%28single-precision%29)))

(event Collision|EventActorBeginOverlap
  (params (OtherActor :type Actor%20Object%20Reference)))

(event EventRuneGeneration
  (bind _runes (Variables|Default|GetRunes))
  (bind _outitem (Utilities|Array|Random _runes))
  (bind _returnvalue (Math|Conversions|ToLinearColor(Color) (.colour_temp _outitem)))
  (Widget|SetVisibility (Variables|/Game/ShikanokoKoshtantan/Blueprints/Interactables/WBP_Temp.WBP_Temp_C|GetButton_0 (Variables|Default|GetNewVar)) "Visible" :!label _label)
  (if (Utilities|Array|ContainsItem (Variables|Default|GetPlayer%20Runes) (.OutItem (Utilities|Array|Random (Variables|Default|GetRunes))))
    (goto _label)
    (else
      (Variables|/Script/UMG.Image|SetColorAndOpacity (Variables|/Game/ShikanokoKoshtantan/Blueprints/Interactables/WBP_Temp.WBP_Temp_C|GetRuneImage (Variables|Default|GetNewVar)) (Utilities|Struct|MakeLinearColor (.r _returnvalue) (.g _returnvalue) (.b _returnvalue) 1.0)))))

(fn ConstructionScript)