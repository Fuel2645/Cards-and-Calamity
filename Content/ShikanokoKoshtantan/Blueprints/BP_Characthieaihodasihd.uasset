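; Player character with movement, look, line-trace interaction with BP_Interactable actors, a minimap and a pause menu toggle whose SetGamePaused values appear inverted.
; GI_test handles health and rune changes, and supplies the rune that ChestOpening shows in the chest widget.
; Debug keys create save objects, save the game instance and restore player location from the "Testing" slot.
; The local GenerateRune random-retry picker is referenced only by unreachable nodes.
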(event Custom|Chest%20Opening
  (bind _returnvalue (Game|GetPlayerController 0))
  (bind _asgi_test (Utilities|Casting|CastToGI_test (Game|GetGameInstance)))
  (bind _random_rune (Default|ActualRuneGeneration _asgi_test))
  (Variables|/Game/ShikanokoKoshtantan/Blueprints/Widegts/WBP_Temp.WBP_Temp_C|SetCurrent%20RUne (Variables|Default|GetChest%20UI) _random_rune)
  (UserInterface|Viewport|AddtoViewport (Variables|Default|GetChest%20UI) 0)
  (Input|SetInputModeUIOnly _returnvalue 0 "DoNotLock" true)
  (Variables|/Script/Engine.PlayerController|SetbShowMouseCursor _returnvalue true))

(event Input|EnhancedActionEvents|EnhancedInputActionIA_Look
  (params (ActionValue :type Vector%202D%20Structure) (ElapsedSeconds :type Float%20%28double-precision%29) (TriggeredSeconds :type Float%20%28double-precision%29) (InputAction :type Input%20Action%20Object%20Reference :default "/Game/JJ-TheBest/Inputs/IA_Look.IA_Look"))
  (Pawn|Input|AddControllerYawInput (.x ActionValue))
  (Pawn|Input|AddControllerPitchInput (.y ActionValue)))

(event Input|EnhancedActionEvents|EnhancedInputActionIA_Movement
  (params (ActionValue :type Vector%202D%20Structure) (ElapsedSeconds :type Float%20%28double-precision%29) (TriggeredSeconds :type Float%20%28double-precision%29) (InputAction :type Input%20Action%20Object%20Reference :default "/Game/JJ-TheBest/Inputs/IA_Movement.IA_Movement"))
  (bind _returnvalue (Pawn|GetControlRotation :!class /Script/Engine.Pawn))
  (Pawn|Input|AddMovementInput (Math|Vector|GetRightVector (Math|Rotator|MakeRotator (.roll _returnvalue) 0.0 (.yaw _returnvalue))) (.x ActionValue) false)
  (Pawn|Input|AddMovementInput (Math|Vector|GetForwardVector (Math|Rotator|MakeRotator 0.0 0.0 (.yaw (Pawn|GetControlRotation :!class /Script/Engine.Pawn)))) (.y ActionValue) false))

(event Input|EnhancedActionEvents|EnhancedInputActionIA_Interact
  (params (ActionValue :type Boolean) (ElapsedSeconds :type Float%20%28double-precision%29) (TriggeredSeconds :type Float%20%28double-precision%29) (InputAction :type Input%20Action%20Object%20Reference :default "/Game/ShikanokoKoshtantan/Blueprints/IA_Interact.IA_Interact"))
  (bind _returnvalue (Transformation|GetActorLocation))
  (bind _outhit (Collision|LineTraceByChannel _returnvalue (+ _returnvalue (* (Transformation|GetActorForwardVector) 1e+06)) "TraceTypeQuery1" false 0 "None"))
  (if (Utilities|ClassIsChildOf (Utilities|GetClass (.hitactor _outhit)) "/Game/ShikanokoKoshtantan/Blueprints/Interactables/BP_Interactable.BP_Interactable_C")
    (Class|BPIInteract|Interact(Message) (.hitactor _outhit))))

(event Input|EnhancedActionEvents|EnhancedInputActionIA_Pause
  (params (ActionValue :type Boolean) (ElapsedSeconds :type Float%20%28double-precision%29) (TriggeredSeconds :type Float%20%28double-precision%29) (InputAction :type Input%20Action%20Object%20Reference :default "/Game/Mateusz/IA_Pause.IA_Pause"))
  (bind _returnvalue (Game|GetPlayerController 0))
  (:Started
    (if (not (Variables|Default|GetPauseOpen))
      (Variables|Default|SetPauseOpen true)
      (bind _returnvalue_2 (UserInterface|CreateWidget "/Game/Mateusz/PauseWidgets/WB_Pause.WB_Pause_C" _returnvalue))
      (bind _output_get (Variables|Default|SetPauseWidget _returnvalue_2))
      (UserInterface|Viewport|AddtoViewport _output_get 0)
      (Input|SetInputModeGameandUI _returnvalue (Variables|Default|GetPauseWidget) "DoNotLock" true false)
      (Variables|/Script/Engine.PlayerController|SetbShowMouseCursor (Game|GetPlayerController 0) true)
      (Game|SetGamePaused false)
      (else
        (Variables|Default|SetPauseOpen false)
        (Widget|RemovefromParent (Variables|Default|GetPauseWidget))
        (Game|SetGamePaused true)
        (Input|SetInputModeGameOnly _returnvalue false)
        (Variables|/Script/Engine.PlayerController|SetbShowMouseCursor (Game|GetPlayerController 0) false)))))

(event EventAddHealth
  (params (Health%20to%20Gain :type Integer))
  (bind _asgi_test (Utilities|Casting|CastToGI_test (Game|GetGameInstance)))
  (Default|ChangeHealth _asgi_test Health%20to%20Gain))

(event EventBeginPlay
  (bind _asplayer_controller (Utilities|Casting|CastToPlayerController (Pawn|GetController)))
  (Utilities|IsValid (PlayerController|LocalPlayerSubsystems|GetEnhancedInputLocalPlayerSubsystem _asplayer_controller)
    (:Is%20Valid
      (Input|AddMappingContext (PlayerController|LocalPlayerSubsystems|GetEnhancedInputLocalPlayerSubsystem _asplayer_controller) "/Game/JJ-TheBest/IMC_Inputs.IMC_Inputs" 0 "(bIgnoreAllPressedKeysUntilRelease=True,bForceImmediately=False,bNotifyUserSettings=False)")
      (bind _returnvalue (UserInterface|CreateWidget "/Game/ShikanokoKoshtantan/Blueprints/Widegts/WBP_Temp.WBP_Temp_C"))
      (Variables|Default|SetChest%20UI _returnvalue)
      (bind _returnvalue_2 (UserInterface|CreateWidget "/Game/ShikanokoKoshtantan/Blueprints/Widegts/WBP_3_Runes.WBP_3_Runes_C"))
      (Variables|Default|Set3%20RUne%20Widget _returnvalue_2)
      (bind _returnvalue_3 (UserInterface|CreateWidget "/Game/JJ-TheBest/WB_MiniMap.WB_MiniMap_C"))
      (UserInterface|Viewport|AddtoViewport _returnvalue_3 0))))

(event EventTick
  (params (DeltaSeconds :type Float%20%28single-precision%29)))

(event Collision|EventActorBeginOverlap
  (params (OtherActor :type Actor%20Object%20Reference)))

(event EventAddRune
  (params (Rune%20to%20add%20 :type ST%20Rune%20Structure))
  (bind _asgi_test (Utilities|Casting|CastToGI_test (Game|GetGameInstance)))
  (Default|AddRune _asgi_test Rune%20to%20add%20))

(event Input|KeyboardEvents|L
  (params (Key :type Key%20Structure :default "None"))
  (:Pressed
    (bind _returnvalue (SaveGame|LoadGamefromSlot "Testing"))
    (Development|PrintString (Utilities|GetDisplayName _returnvalue))
    (bind _asbp_save_game_obj (Utilities|Casting|CastToBP_SaveGameOBJ _returnvalue))
    (bind _asgi_test (Utilities|Casting|CastToGI_test (Variables|/Game/ShikanokoKoshtantan/Blueprints/BP_SaveGameOBJ.BP_SaveGameOBJ_C|GetSaved%20Instance _asbp_save_game_obj)))
    (Transformation|SetActorLocation (Game|GetPlayerCharacter 0) (Variables|/Game/Patryk_Klich/GameMode/GI_test.GI_test_C|GetPlayerLocation _asgi_test) false true)))

(event Input|KeyboardEvents|J
  (params (Key :type Key%20Structure :default "None"))
  (:Pressed
    (bind _returnvalue (SaveGame|CreateSaveGameObject "/Game/ShikanokoKoshtantan/Blueprints/BP_SaveGameOBJ.BP_SaveGameOBJ_C"))
    (Default|SaveGame _returnvalue (Game|GetGameInstance) "Testing")))

(event Input|KeyboardEvents|NumPadSeven
  (params (Key :type Key%20Structure :default "None"))
  (:Pressed
    (bind _returnvalue (SaveGame|CreateSaveGameObject "/Game/ShikanokoKoshtantan/Blueprints/BP_MasterSaveGame.BP_MasterSaveGame_C"))
    (Default|Intialise _returnvalue)))

(fn ConstructionScript)

(fn GenerateRune
  (LocalVariables|SetRuneCOunt 0)
  (bind _asgi_test (Utilities|Casting|CastToGI_test (Game|GetGameInstance)))
  (bind _output_get (Variables|Default|SetRandRune (.OutItem (Utilities|Array|Random (Variables|/Game/Patryk_Klich/GameMode/GI_test.GI_test_C|GetRunes _asgi_test))) :!label _label))
  (if (Utilities|Array|ContainsItem (Variables|/Game/Patryk_Klich/GameMode/GI_test.GI_test_C|GetPlayer%20Runes _asgi_test) _output_get)
    (bind _result (Math|Integer|IncrementInt (LocalVariables|GetRuneCOunt))
      (:%20%20
        (if (== _result (Utilities|Array|Length (Variables|/Game/Patryk_Klich/GameMode/GI_test.GI_test_C|GetRunes _asgi_test)))
          (return "" false)
          (else
            (goto _label)))))
    (else
      (return _output_get true))))

(fn RuneGeneration
  (return))