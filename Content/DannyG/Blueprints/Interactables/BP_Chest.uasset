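; BP_Chest is an interactable chest that triggers a chest-opening response on the player character.
; Its Interact event passes through a DoOnce, so only the first interaction takes effect.
; It then casts player character 0 to BP_Characthieaihodasihd and calls ChestOpening, leaving the opening logic to that character Blueprint.
; The chest has no other active logic of its own.
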(event EventBeginPlay
  (|CallParentFunction) ; This node is disabled and will not be called.\nDrag off pins to build functionality.
)

(event Collision|EventActorBeginOverlap
  (params (OtherActor :type Actor%20Object%20Reference))
  (|CallParentFunction OtherActor) ; This node is disabled and will not be called.\nDrag off pins to build functionality.
)

(event EventTick
  (params (DeltaSeconds :type Float%20%28single-precision%29))
  (|CallParentFunction DeltaSeconds) ; This node is disabled and will not be called.\nDrag off pins to build functionality.
)

(event EventInteract
  (Utilities|FlowControl|DoOnce false
    (:Completed
      (bind _asbp_characthieaihodasihd (Utilities|Casting|CastToBP_Characthieaihodasihd (Game|GetPlayerCharacter 0)))
      (Default|ChestOpening _asbp_characthieaihodasihd))))

(fn ConstructionScript
  (|CallParentFunction))