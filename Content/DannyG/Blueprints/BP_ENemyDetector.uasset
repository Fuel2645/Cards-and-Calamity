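; BP_ENemyDetector checks whether every BP_TestingDummyAI enemy in the level is dead and reports that to the player controller.
; Initialise stores a HasKey flag and caches all dummy AI actors found at that moment.
; DeathCheck scans the cached list, stopping at the first living enemy; if none remain, it sends DeathCheckMessage with HasKey to player controller 0.
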(event Custom|Initialise
  (params (HasKey :type Boolean))
  (Variables|Default|SetHasKey HasKey)
  (bind _outactors (Actor|GetAllActorsOfClass "/Game/Patryk_Klich/TestingAi/BP_TestingDummyAI.BP_TestingDummyAI_C"))
  (Variables|Default|SetEnemies _outactors))

(event EventDeathCheck
  (params (NeedKey :type Boolean))
  (Variables|Default|SetAllDead true)
  (bind _array_element (Utilities|Array|ForEachLoopwithBreak (Variables|Default|GetEnemies) :!label _label)
    (:LoopBody
      (bind _asbp_testing_dummy_ai (Utilities|Casting|CastToBP_TestingDummyAI _array_element))
      (if (not (Variables|/Game/Patryk_Klich/TestingAi/BP_TestingDummyAI.BP_TestingDummyAI_C|GetIsDead _asbp_testing_dummy_ai))
        (Variables|Default|SetAllDead false)
        (goto _label Break)))
    (:Completed
      (if (Variables|Default|GetAllDead)
        (Class|BPIDamageTransfer|DeathCheck(Message) (Game|GetPlayerController 0) (Variables|Default|GetHasKey))))))

(fn ConstructionScript)