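; BP_PatrolPath is a spline-based patrol path that supplies world-space points for patrolling.
; GetPatrolPoint steps CurrentIndex by Direction, then returns that spline point as Start and the last spline point as End.
; PatrolPoints forwards both values from GetPatrolPoint, so calling it can also change the index.
; The index has no active bounds or reversal logic: its zero check is unconnected, and GetPatrolPath is an empty stub.
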(fn ConstructionScript)

(fn GetPatrolPoint
  (bind _output_get (Variables|Default|SetCurrent%20Index (+ (Variables|Default|GetCurrent%20Index) (Variables|Default|GetDirection))))
  (return (Spline|GetLocationatSplinePoint (Variables|Default|GetSpline) _output_get "World") (Spline|GetLocationatSplinePoint (Variables|Default|GetSpline) (- (Spline|GetNumberOfSplinePoints (Variables|Default|GetSpline)) 1) "World")))

(fn GetPatrolPath
  (return 0))

(fn PatrolPoints
  (bind (_start _end) (CallFunction|GetPatrolPoint))
  (return _start _end))