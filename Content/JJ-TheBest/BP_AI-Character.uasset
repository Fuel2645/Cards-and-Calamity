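; AI enemy character that detects the player by sight and by proximity.
; PawnSensing sets the "SeePlayer?" blackboard bool when it sees the player character class, and nothing here clears it.
; On player overlap, its sphere saves the player's location to the GI_test game instance and passes it this enemy's layout and original reference.
; Setter events supply patrol path, layout and reference; construction caches the spawn location.
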(event OnComponentBeginOverlap(Sphere)
  (params (OverlappedComponent :type Primitive%20Component%20Object%20Reference) (OtherActor :type Actor%20Object%20Reference) (OtherComp :type Primitive%20Component%20Object%20Reference) (OtherBodyIndex :type Integer) (bFromSweep :type Boolean) (SweepResult :type Hit%20Result%20Structure%20%28by%20ref%29))
  (if (== OtherActor (Game|GetPlayerCharacter 0))
    (bind _asgi_test (Utilities|Casting|CastToGI_test (Game|GetGameInstance)))
    (Variables|/Game/Patryk_Klich/GameMode/GI_test.GI_test_C|SetPlayerLocation _asgi_test (Transformation|GetActorLocation (Game|GetPlayerCharacter 0)))
    (Default|SetEnemies _asgi_test (Variables|Default|GetEnemy%20Layout) (Variables|Default|GetOriginal%20Ref))))

(event OnSeePawn(PawnSensing)
  (params (Pawn :type Pawn%20Object%20Reference))
  (Utilities|Casting|CastToBP_Characthieaihodasihd Pawn)
  (AI|Components|Blackboard|SetValueasBool (AI|GetBlackboard (AI|GetAIController self)) (Utilities|Name|MakeLiteralName "SeePlayer?") true))

(event Custom|Set%20Patrol
  (params (Patrol%20Point :type Actor%20Object%20Reference))
  (Variables|Default|SetPatrolPath Patrol%20Point))

(event Custom|Set%20Ref
  (params (AI%20ref :type BP%20AI-Character%20Object%20Reference))
  (Variables|Default|SetOriginal%20Ref AI%20ref))

(event Custom|Set%20Layout
  (params (Layout :type Map%20of%20Integers%20to%20Names))
  (Variables|Default|SetEnemy%20Layout Layout))

(event EventBeginPlay)

(fn ConstructionScript
  (Variables|Default|SetOriginal%20Locatcion (Transformation|GetActorLocation)))

(fn GetPatrolPath
  (return (Variables|Default|GetPatrolPath)))

(fn PatrolPoints
  (return "0, 0, 0" "0, 0, 0"))