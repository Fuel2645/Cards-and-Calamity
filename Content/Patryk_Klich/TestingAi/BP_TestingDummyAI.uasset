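; BP_TestingDummyAI is a test enemy for turn-based combat, selected on the player controller by clicking its cube.
; TransferDataTableIndex loads its stats and material from DT_Enemies and initializes the health bar widget.
; Attack applies damage minus reduction and destroys it at zero HP, while AIAttack randomly damages the player controller's HP unless stunned.
; EndTurnStatus ticks burn, stun and bleed, routing damage-over-time through Attack.
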(event OnClicked(Cube)
  (params (TouchedComponent :type Primitive%20Component%20Object%20Reference) (ButtonPressed :type Key%20Structure :default "None"))
  (Class|BPIDamageTransfer|Select(Message) (Game|GetPlayerController 0) self))

(event Custom|Death
  (Actor|DestroyActor))

(event Custom|EndTurnStatus
  (for _index (range 0 2)
    (Variables|Default|SetStatusType _index)
    (if (.Value (Utilities|Map|Find (Variables|Default|GetstatusEffects) _index))
      (switch int _index
        (:0
          (Development|PrintString "burn")
          (if (<= (Variables|StatusTicks|GetBurnTicks) 0)
            (Utilities|Map|Add (Variables|Default|GetstatusEffects) (Variables|Default|GetStatusType) false)
            (else
              (CallFunction|Attack (Variables|Default|GetBurn%20Damage))
              (Math|Integer|DecrementInt (Variables|StatusTicks|GetBurnTicks)))))
        (:1
          (Development|PrintString "stun")
          (if (<= (Variables|StatusTicks|GetStun%20Ticks) 0)
            (Utilities|Map|Add (Variables|Default|GetstatusEffects) (Variables|Default|GetStatusType) false)
            (else
              (Math|Integer|DecrementInt (Variables|StatusTicks|GetStun%20Ticks)))))
        (:2
          (Development|PrintString "bleed")
          (if (<= (Variables|StatusTicks|GetBleed%20Ticks) 0)
            (Utilities|Map|Add (Variables|Default|GetstatusEffects) (Variables|Default|GetStatusType) false)
            (else
              (CallFunction|Attack (Variables|Default|GetBleedDamage))
              (Math|Integer|DecrementInt (Variables|StatusTicks|GetBleed%20Ticks)))))))))

(event EventBeginPlay
  (bind _asbp_player_control_combat (Utilities|Casting|CastToBP_PlayerControlCombat (Game|GetPlayerController 0)))
  (Variables|Default|SetPCREF _asbp_player_control_combat))

(event Collision|EventActorBeginOverlap
  (params (OtherActor :type Actor%20Object%20Reference)))

(event EventTick
  (params (DeltaSeconds :type Float%20%28single-precision%29)))

(event EventTransferDataTableIndex
  (params (RowName :type Name :default "None"))
  (bind _returnvalue (Utilities|GetDataTableRow "/Game/ShikanokoKoshtantan/DataValues/Enemies/DT_Enemies.DT_Enemies" RowName)
    (:then
      (bind _output_get (Variables|Default|SetMin%20Damage (.MinDamage (Utilities|Struct|BreakST_Enemies _returnvalue))))
      (bind _output_get_2 (Variables|Default|SetMax%20Damage (.MaxDamage (Utilities|Struct|BreakST_Enemies _returnvalue))))
      (bind _output_get_3 (Variables|Default|SetHp (.Health (Utilities|Struct|BreakST_Enemies _returnvalue))))
      (Variables|Default|SetMaxHP (.Health (Utilities|Struct|BreakST_Enemies _returnvalue)))
      (Variables|Default|SetDodgeChance (.DodgeChance (Utilities|Struct|BreakST_Enemies _returnvalue)))
      (Rendering|Material|SetMaterial (Variables|Default|GetCube) 0 (.MemberVar_18 (Utilities|Struct|BreakST_Enemies _returnvalue)))
      (Development|PrintString (Utilities|String|Append (Utilities|String|ToString(Name) RowName) " has " (Utilities|String|ToString(Integer) _output_get) " min attack " (Utilities|String|ToString(Integer) _output_get_2) " max attack and " (Utilities|String|ToString(Integer) _output_get_3) " HP") true true "(R=0.000000,G=0.660000,B=1.000000,A=1.000000)" 3.0)
      (CallFunction|SetWidgetMaxHP)
      (CallFunction|UpdateWidgetHP))))

(event EventAttack
  (params (DamageAmount :type Integer))
  (bind _output_get (Variables|Default|SetHp (- (Variables|Default|GetHp) (- DamageAmount (Variables|Default|GetDamageReduction)))))
  (if (<= _output_get 0)
    (Actor|DestroyActor)
    (else
      (CallFunction|UpdateWidgetHP))))

(event EventAIAttack
  (bind _pcref (Variables|Default|GetPCREF))
  (if (<= (Variables|StatusTicks|GetStun%20Ticks) 0)
    (Variables|/Game/Patryk_Klich/GameMode/BP_PlayerControlCombat.BP_PlayerControlCombat_C|SetHP _pcref (- (Variables|/Game/Patryk_Klich/GameMode/BP_PlayerControlCombat.BP_PlayerControlCombat_C|GetHP _pcref) (Math|Random|RandomIntegerinRange (Variables|Default|GetMin%20Damage) (Variables|Default|GetMax%20Damage))))))

(fn ConstructionScript)

(fn UpdateWidgetHP
  (bind _aswb_health (Utilities|Casting|CastToWB_Health (UserInterface|GetUserWidgetObject (Variables|Default|GetHealthBar))))
  (Variables|/Game/Patryk_Klich/TestingAi/WB_Health.WB_Health_C|SetHP _aswb_health (Variables|Default|GetHp))
  (return))

(fn SetWidgetMaxHP
  (bind _aswb_health (Utilities|Casting|CastToWB_Health (UserInterface|GetUserWidgetObject (Variables|Default|GetHealthBar))))
  (Variables|/Game/Patryk_Klich/TestingAi/WB_Health.WB_Health_C|SetMaxHP _aswb_health (Variables|Default|GetMaxHP)))