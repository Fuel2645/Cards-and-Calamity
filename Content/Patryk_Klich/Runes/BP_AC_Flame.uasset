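; Flame rune component that applies a burn to the selected enemy.
; Its Rune Action stores the enemy, copies the rune's tick count and damage into that enemy's burn variables and sets status effect 0 to true.
; It then immediately calls Attack on the enemy with the burn damage.
; The component only writes the burn state, with no tick logic of its own.
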(event EventBeginPlay
  (|CallParentFunction) ; This node is disabled and will not be called.\nDrag off pins to build functionality.
)

(event EventTick
  (params (DeltaSeconds :type Float%20%28single-precision%29))
  (|CallParentFunction DeltaSeconds) ; This node is disabled and will not be called.\nDrag off pins to build functionality.
)

(fn RuneAction
  (params (SelectedEnemy :type BP%20Testing%20Dummy%20AI%20Object%20Reference))
  (bind _output_get (LocalVariables|SetSelected%20Enemy SelectedEnemy))
  (Variables|/Game/Patryk_Klich/TestingAi/BP_TestingDummyAI.BP_TestingDummyAI_C|SetBurnTicks _output_get (Variables|Default|GetNumberOfTicks))
  (Utilities|Map|Add (Variables|/Game/Patryk_Klich/TestingAi/BP_TestingDummyAI.BP_TestingDummyAI_C|GetstatusEffects (LocalVariables|GetSelected%20Enemy)) 0 true)
  (bind _output_get_2 (Variables|/Game/Patryk_Klich/TestingAi/BP_TestingDummyAI.BP_TestingDummyAI_C|SetBurn%20Damage (LocalVariables|GetSelected%20Enemy) (Variables|Default|GetDamage)))
  (Default|Attack (LocalVariables|GetSelected%20Enemy) _output_get_2))