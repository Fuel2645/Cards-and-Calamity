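; Guard rune component that grants the player armor in combat when its rune action fires.
; RuneAction casts player controller 0 to BP_PlayerControlCombat and adds ArmorAmount to its Armor, capped at MaxArmor.
; The selected enemy and rune index inputs are unused, and the event graph holds only disabled stubs.
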(event EventBeginPlay
  (|CallParentFunction) ; This node is disabled and will not be called.\nDrag off pins to build functionality.
)

(event EventTick
  (params (DeltaSeconds :type Float%20%28single-precision%29))
  (|CallParentFunction DeltaSeconds) ; This node is disabled and will not be called.\nDrag off pins to build functionality.
)

(fn RuneAction
  (params (SelectedEnemy :type BP%20Testing%20Dummy%20AI%20Object%20Reference) (RuneIndex :type Integer))
  (bind _asbp_player_control_combat (Utilities|Casting|CastToBP_PlayerControlCombat (Game|GetPlayerController 0)))
  (if (> (+ (Variables|/Game/Patryk_Klich/GameMode/BP_PlayerControlCombat.BP_PlayerControlCombat_C|GetArmor _asbp_player_control_combat) (Variables|Default|GetArmorAmount)) (Variables|/Game/Patryk_Klich/GameMode/BP_PlayerControlCombat.BP_PlayerControlCombat_C|GetMaxArmor _asbp_player_control_combat))
    (Variables|/Game/Patryk_Klich/GameMode/BP_PlayerControlCombat.BP_PlayerControlCombat_C|SetArmor _asbp_player_control_combat (Variables|/Game/Patryk_Klich/GameMode/BP_PlayerControlCombat.BP_PlayerControlCombat_C|GetMaxArmor _asbp_player_control_combat))
    (else
      (Variables|/Game/Patryk_Klich/GameMode/BP_PlayerControlCombat.BP_PlayerControlCombat_C|SetArmor _asbp_player_control_combat (+ (Variables|/Game/Patryk_Klich/GameMode/BP_PlayerControlCombat.BP_PlayerControlCombat_C|GetArmor _asbp_player_control_combat) (Variables|Default|GetArmorAmount))))))