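; Detonate rune component that cashes in the remaining bleed and burn on a selected enemy as immediate damage.
; Its rune action multiplies each effect's remaining ticks by its per-tick damage and deals the total in a single attack.
; If the enemy is still valid afterwards, it zeroes the consumed ticks, flags those status effects false and calls the enemy's effect clearing.
; An enemy with neither effect is left untouched.
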(event EventBeginPlay
  (|CallParentFunction) ; This node is disabled and will not be called.\nDrag off pins to build functionality.
)

(event EventTick
  (params (DeltaSeconds :type Float%20%28single-precision%29))
  (|CallParentFunction DeltaSeconds) ; This node is disabled and will not be called.\nDrag off pins to build functionality.
)

(fn RuneAction
  (params (SelectedEnemy :type BP%20Testing%20Dummy%20AI%20Object%20Reference) (RuneIndex :type Integer))
  (LocalVariables|SetSelected%20Enemy SelectedEnemy)
  (Variables|Default|SetBleedTicks (Variables|/Game/Patryk_Klich/TestingAi/BP_TestingDummyAI.BP_TestingDummyAI_C|GetBleed%20Ticks SelectedEnemy))
  (Variables|Default|SetBurnTicks (Variables|/Game/Patryk_Klich/TestingAi/BP_TestingDummyAI.BP_TestingDummyAI_C|GetBurnTicks SelectedEnemy))
  (Variables|Default|SetBleedDamage (Variables|/Game/Patryk_Klich/TestingAi/BP_TestingDummyAI.BP_TestingDummyAI_C|GetBleedDamage SelectedEnemy))
  (Variables|Default|SetBurnDamage (Variables|/Game/Patryk_Klich/TestingAi/BP_TestingDummyAI.BP_TestingDummyAI_C|GetBurn%20Damage SelectedEnemy))
  (if (and (> (Variables|Default|GetBleedTicks) 0) (> (Variables|Default|GetBurnTicks) 0))
    (Default|Attack (LocalVariables|GetSelected%20Enemy) (+ (* (Variables|Default|GetBurnTicks) (Variables|Default|GetBurnDamage)) (* (Variables|Default|GetBleedTicks) (Variables|Default|GetBleedDamage))))
    (Utilities|IsValid (LocalVariables|GetSelected%20Enemy)
      (:Is%20Valid
        (Variables|/Game/Patryk_Klich/TestingAi/BP_TestingDummyAI.BP_TestingDummyAI_C|SetBurnTicks (LocalVariables|GetSelected%20Enemy) 0)
        (Variables|/Game/Patryk_Klich/TestingAi/BP_TestingDummyAI.BP_TestingDummyAI_C|SetBleed%20Ticks (LocalVariables|GetSelected%20Enemy) 0)
        (Utilities|Map|Add (Variables|/Game/Patryk_Klich/TestingAi/BP_TestingDummyAI.BP_TestingDummyAI_C|GetstatusEffects (LocalVariables|GetSelected%20Enemy)) 0 false)
        (Utilities|Map|Add (Variables|/Game/Patryk_Klich/TestingAi/BP_TestingDummyAI.BP_TestingDummyAI_C|GetstatusEffects (LocalVariables|GetSelected%20Enemy)) 2 false)
        (Default|ClearEffects (LocalVariables|GetSelected%20Enemy) :!label _label)))
    (elif (> (Variables|Default|GetBleedTicks) 0)
      (Default|Attack (LocalVariables|GetSelected%20Enemy) (* (Variables|Default|GetBleedTicks) (Variables|Default|GetBleedDamage)))
      (Utilities|IsValid (LocalVariables|GetSelected%20Enemy)
        (:Is%20Valid
          (Variables|/Game/Patryk_Klich/TestingAi/BP_TestingDummyAI.BP_TestingDummyAI_C|SetBleed%20Ticks (LocalVariables|GetSelected%20Enemy) 0)
          (Utilities|Map|Add (Variables|/Game/Patryk_Klich/TestingAi/BP_TestingDummyAI.BP_TestingDummyAI_C|GetstatusEffects (LocalVariables|GetSelected%20Enemy)) 2 false)
          (goto _label)))
      (elif (> (Variables|Default|GetBurnTicks) 0)
        (Default|Attack (LocalVariables|GetSelected%20Enemy) (* (Variables|Default|GetBurnTicks) (Variables|Default|GetBurnDamage)))
        (Utilities|IsValid (LocalVariables|GetSelected%20Enemy)
          (:Is%20Valid
            (Variables|/Game/Patryk_Klich/TestingAi/BP_TestingDummyAI.BP_TestingDummyAI_C|SetBurnTicks (LocalVariables|GetSelected%20Enemy) 0)
            (Utilities|Map|Add (Variables|/Game/Patryk_Klich/TestingAi/BP_TestingDummyAI.BP_TestingDummyAI_C|GetstatusEffects (LocalVariables|GetSelected%20Enemy)) 0 false)
            (goto _label)))))))