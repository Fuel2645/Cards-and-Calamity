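; BP_AC_Stun is a rune effect that stuns the selected enemy.
; Its Rune Action stores the passed enemy and sets that enemy's StunTicks from the NumberOfTicks variable.
; It then flags the stun in the enemy's StatusEffects collection and calls StatusEffectDisplay on that enemy.
; The rune only applies the status; it has no active BeginPlay or Tick logic.
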(event EventBeginPlay
  (|CallParentFunction) ; This node is disabled and will not be called.\nDrag off pins to build functionality.
)

(event EventTick
  (params (DeltaSeconds :type Float%20%28single-precision%29))
  (|CallParentFunction DeltaSeconds) ; This node is disabled and will not be called.\nDrag off pins to build functionality.
)

(fn RuneAction
  (params (SelectedEnemy :type BP%20Testing%20Dummy%20AI%20Object%20Reference) (RuneIndex :type Integer))
  (bind _output_get (Variables|Default|SetSelected%20Enemy SelectedEnemy))
  (Variables|/Game/Patryk_Klich/TestingAi/BP_TestingDummyAI.BP_TestingDummyAI_C|SetStun%20Ticks _output_get (Variables|Default|GetNumberOfTicks))
  (Utilities|Map|Add (Variables|/Game/Patryk_Klich/TestingAi/BP_TestingDummyAI.BP_TestingDummyAI_C|GetstatusEffects (Variables|Default|GetSelected%20Enemy)) 1 true)
  (Default|StatusEffectDisplay (Variables|Default|GetSelected%20Enemy)))