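; BP_AC_PhysicalAttack is the "Strike" combat rune, a physical attack on the selected enemy with a cooldown of 2.
; Its action rolls damage between MinAttack and MaxAttack, multiplies it by CritDamage on a crit, and passes it to the enemy's Attack.
; A crit needs a 1–4 roll above the player controller's CritChance, which resets to 4 afterwards, so crits require that value to be lowered beforehand.
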(event EventBeginPlay
  (|CallParentFunction) ; This node is disabled and will not be called.\nDrag off pins to build functionality.
)

(event EventTick
  (params (DeltaSeconds :type Float%20%28single-precision%29))
  (|CallParentFunction DeltaSeconds) ; This node is disabled and will not be called.\nDrag off pins to build functionality.
)

(fn RuneAction
  (params (SelectedEnemy :type BP%20Testing%20Dummy%20AI%20Object%20Reference))
  (bind _minattack (Variables|Default|GetMinAttack))
  (bind _maxattack (Variables|Default|GetMaxAttack))
  (bind _returnvalue (Math|Random|RandomIntegerinRange _minattack _maxattack))
  (LocalVariables|SetEnemy SelectedEnemy)
  (bind _asbp_player_control_combat (Utilities|Casting|CastToBP_PlayerControlCombat (Game|GetPlayerController 0)))
  (Variables|Default|SetPlayer _asbp_player_control_combat)
  (if (> (Math|Random|RandomIntegerinRange 1 4) (Variables|/Game/Patryk_Klich/GameMode/BP_PlayerControlCombat.BP_PlayerControlCombat_C|GetCritChance _asbp_player_control_combat))
    (Development|PrintString "CRIT")
    (Default|Attack (LocalVariables|GetEnemy) (* _returnvalue (Variables|Default|GetCritDamage)))
    (else
      (Default|Attack (LocalVariables|GetEnemy) _returnvalue)))
  (Variables|/Game/Patryk_Klich/GameMode/BP_PlayerControlCombat.BP_PlayerControlCombat_C|SetCritChance (Variables|Default|GetPlayer) 4))

(fn SetRuneName
  (Variables|Default|SetRuneName "Strike"))

(fn SetRuneCooldown
  (Variables|Default|SetCooldown 2))