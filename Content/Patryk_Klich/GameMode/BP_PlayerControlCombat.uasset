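; BP_PlayerControlCombat is the player controller for combat, handling the combat HUD, enemy selection and rune use.
; On BeginPlay it shows the cursor, sets Game and UI input and creates the WB_CombatHUD widget.
; Select stores the chosen enemy and refreshes the HUD buttons based on whether action points are zero.
; RuneExecution picks a BP_AC_RuneBase component by index and runs its RuneAction on the selected enemy.
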(event EventBeginPlay
  (bind _self self)
  (Input|SetInputModeGameandUI _self 0 "DoNotLock" false false)
  (Variables|/Script/Engine.PlayerController|SetbShowMouseCursor _self true)
  (bind _returnvalue (UserInterface|CreateWidget "/Game/Patryk_Klich/HUD/WB_CombatHUD.WB_CombatHUD_C"))
  (bind _output_get (Variables|Default|SetHUD _returnvalue))
  (UserInterface|Viewport|AddtoViewport _output_get 0))

(event EventSelect
  (params (Selected%20Enemy :type BP%20Testing%20Dummy%20AI%20Object%20Reference))
  (bind _hud (Variables|Default|GetHUD))
  (Variables|Default|SetSelected%20Enemy Selected%20Enemy)
  (Default|UpdateButtonEnableStatus _hud (== (Variables|/Game/Patryk_Klich/HUD/WB_CombatHUD.WB_CombatHUD_C|GetActionPoints _hud) 0)))

(event EventRuneExecution
  (params (RuneIndex :type Integer))
  (Default|RuneAction (Utilities|Array|Get(acopy) (Actor|GetComponentsByClass self "/Game/ShikanokoKoshtantan/Rune_Components/BP_AC_RuneBase.BP_AC_RuneBase_C") RuneIndex) (Variables|Default|GetSelected%20Enemy)))

(fn ConstructionScript)