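; GM_Combat is a combat game mode that sets up and drives the enemy side of battles.
; TransferData reads the GI_test game instance's enemy map by array index and passes each value to the matching enemy in EnemyArrayGM as a data table index.
; AIAttack loops over the valid enemies, having each one attack and then run its end-turn status step.
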(event Custom|TransferData
  (bind _asgi_test (Utilities|Casting|CastToGI_test (Game|GetGameInstance)))
  (for (_array_element _array_index) (Variables|Default|GetEnemyArrayGM)
    (Default|TransferDataTableIndex _array_element (.Value (Utilities|Map|Find (Variables|/Game/Patryk_Klich/GameMode/GI_test.GI_test_C|GetEnemyArray _asgi_test) _array_index)))))

(event EventBeginPlay)

(event EventAIAttack
  (for _array_element (Variables|Default|GetEnemyArrayGM)
    (Utilities|IsValid _array_element
      (:Is%20Valid
        (Default|AIAttack _array_element)
        (Default|EndTurnStatus _array_element)))))

(fn ConstructionScript)